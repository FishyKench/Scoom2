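; BP_MovingPlatformWithJumpad is a platform actor that moves between two point components, Point1 and Point2.
; On BeginPlay it plays MovementTimeline at a rate set by Speed.
; Each update lerps the Platform's world location between the points using the timeline's Alpha, teleporting without sweep.
; Despite the name, its graphs contain no jump pad logic.
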(event EventBeginPlay
  (Components|Timeline|SetPlayRate (Variables|Default|GetMovementTimeline) (/ (Variables|Default|GetSpeed) 1.0))
  (bind _alpha (Timeline|MovementTimeline Play)
    (:Update
      (Transformation|SetWorldLocation (Variables|Default|GetPlatform) (Math|Vector|Lerp(Vector) (Transformation|GetWorldLocation (Variables|Default|GetPoint1)) (Transformation|GetWorldLocation (Variables|Default|GetPoint2)) _alpha) false true))))

(fn ConstructionScript)