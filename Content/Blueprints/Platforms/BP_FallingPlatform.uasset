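; Falling platform that drops after a player steps on it, then resets to its starting spot.
; A Trigger overlap from an actor tagged Player waits a configurable HowFastToFall delay, then enables physics on the StaticMesh so it falls.
; After a few seconds it stops simulating, briefly disables collision, teleports to the transform cached at BeginPlay and restores collision.
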(event OnComponentBeginOverlap(Trigger)
  (params (OverlappedComponent :type Primitive%20Component%20Object%20Reference) (OtherActor :type Actor%20Object%20Reference) (OtherComp :type Primitive%20Component%20Object%20Reference) (OtherBodyIndex :type Integer) (bFromSweep :type Boolean) (SweepResult :type Hit%20Result%20Structure%20%28by%20ref%29))
  (bind _staticmesh (Variables|Default|GetStaticMesh))
  (if (Actor|ActorHasTag OtherActor "Player")
    (Utilities|FlowControl|Delay (Variables|Default|GetHowFastToFall))
    (Physics|SetSimulatePhysics (Variables|Default|GetStaticMesh) true)
    (Utilities|FlowControl|Delay 3.0)
    (Physics|SetSimulatePhysics _staticmesh false)
    (Collision|SetCollisionEnabled (Variables|Default|GetStaticMesh) "NoCollision")
    (Utilities|FlowControl|Delay 0.2)
    (Transformation|SetWorldTransform _staticmesh (Variables|Default|GetDefaultTransform) false true)
    (Collision|SetCollisionEnabled (Variables|Default|GetStaticMesh) "QueryAndPhysics")))

(event EventBeginPlay
  (Variables|Default|SetDefaultTransform (Transformation|GetWorldTransform (Variables|Default|GetStaticMesh))))

(fn ConstructionScript)