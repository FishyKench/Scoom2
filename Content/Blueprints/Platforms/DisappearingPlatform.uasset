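; A disappearing platform that switches its Cube between visible and solid, and hidden with no collision.
; On BeginPlay, both timelines take their play rate from Speed, and StartOn selects whether ONOFFON or OFFONOFF plays.
; Each update of the chosen timeline's Timer track drives the toggle, with positive values showing the platform and enabling query and physics collision.
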(event EventBeginPlay
  (bind _cube (Variables|Default|GetCube))
  (bind _cube_2 (Variables|Default|GetCube))
  (bind _cube_3 (Variables|Default|GetCube))
  (bind _cube_4 (Variables|Default|GetCube))
  (Components|Timeline|SetPlayRate (Variables|Default|GetON/OFF/ON) (Variables|Default|GetSpeed))
  (Components|Timeline|SetPlayRate (Variables|Default|GetOFF/ON/OFF) (Variables|Default|GetSpeed))
  (if (Variables|Default|GetStartOn?)
    (bind _timer (Timeline|ON/OFF/ON Play)
      (:Update
        (if (> _timer 0.0)
          (Rendering|SetVisibility _cube_4 true false)
          (Collision|SetCollisionEnabled _cube_4 "QueryAndPhysics")
          (else
            (Rendering|SetVisibility _cube_3 false false)
            (Collision|SetCollisionEnabled _cube_3 "NoCollision")))))
    (else
      (bind _timer_2 (Timeline|OFF/ON/OFF Play)
        (:Update
          (if (> _timer_2 0.0)
            (Rendering|SetVisibility _cube_2 true false)
            (Collision|SetCollisionEnabled _cube_2 "QueryAndPhysics")
            (else
              (Rendering|SetVisibility _cube false false)
              (Collision|SetCollisionEnabled _cube "NoCollision"))))))))

(fn ConstructionScript)