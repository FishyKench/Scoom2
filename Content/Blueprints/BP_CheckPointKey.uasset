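; BP_CheckPointKey is a key pickup that unlocks the portal of the BP_NoobDoorTeleporter.
; A Timeline started on BeginPlay animates the mesh's height and yaw around its starting Z.
; When a Player-tagged actor overlaps the box, it sets HasKey on the first teleporter found and activates its portal visual.
; It then plays a sound at world origin, triggers the game mode's teleporter cutscene and destroys itself.
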(event OnComponentBeginOverlap(Box)
  (params (OverlappedComponent :type Primitive%20Component%20Object%20Reference) (OtherActor :type Actor%20Object%20Reference) (OtherComp :type Primitive%20Component%20Object%20Reference) (OtherBodyIndex :type Integer) (bFromSweep :type Boolean) (SweepResult :type Hit%20Result%20Structure%20%28by%20ref%29))
  (if (Actor|ActorHasTag OtherActor "Player")
    (bind _returnvalue (Actor|GetActorOfClass "/Game/Blueprints/BP_NoobDoorTeleporter.BP_NoobDoorTeleporter_C"))
    (bind _output_get (Variables|Default|SetNoobDoor _returnvalue))
    (Variables|/Game/Blueprints/BP_NoobDoorTeleporter.BP_NoobDoorTeleporter_C|SetHasKey? _output_get true)
    (Default|ActivatePortalVisual _output_get)
    (Audio|PlaySoundatLocation "/Game/SFX/PillyPickUp.PillyPickUp" "0, 0, 0" "0, 0, 0" 1.0 1.0 0.0 0 0 0 0)
    (bind _asbp_third_person_game_mode (Utilities|Casting|CastToBP_ThirdPersonGameMode (Game|GetGameMode)))
    (Default|PlayTeleporterCutscene _asbp_third_person_game_mode)
    (Actor|DestroyActor)))

(event EventBeginPlay
  (bind _keymesh (Variables|Default|GetKeyMesh))
  (bind _returnvalue (Transformation|GetWorldLocation _keymesh))
  (Variables|Default|SetDefaultKeyZLocation (.z (Transformation|GetWorldLocation (Variables|Default|GetKeyMesh))))
  (bind (_direction _rotation _position) (Timeline|Timeline Play)
    (:Update
      (Transformation|SetWorldLocationAndRotation _keymesh (Math|Vector|MakeVector (.x _returnvalue) (.y _returnvalue) (+ (Variables|Default|GetDefaultKeyZLocation) _position)) (Math|Rotator|MakeRotator 0.0 0.0 _rotation) false false))))

(fn ConstructionScript)