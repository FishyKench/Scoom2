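; BP_Pill is a collectible pickup that increases the game mode's pill count when the player touches it.
; On BeginPlay it stores the pill's height, then plays a timeline that drives a Z offset and yaw to animate it.
; A sphere overlap with an actor tagged Player calls IncreasePill on BP_ThirdPersonGameMode, then destroys the pickup.
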(event OnComponentBeginOverlap(Sphere)
  (params (OverlappedComponent :type Primitive%20Component%20Object%20Reference) (OtherActor :type Actor%20Object%20Reference) (OtherComp :type Primitive%20Component%20Object%20Reference) (OtherBodyIndex :type Integer) (bFromSweep :type Boolean) (SweepResult :type Hit%20Result%20Structure%20%28by%20ref%29))
  (if (Actor|ActorHasTag OtherActor "Player")
    (bind _asbp_third_person_game_mode (Utilities|Casting|CastToBP_ThirdPersonGameMode (Game|GetGameMode)))
    (Default|IncreasePill _asbp_third_person_game_mode)
    (Actor|DestroyActor)))

(event EventBeginPlay
  (bind _pill (Variables|Default|GetPill))
  (bind _returnvalue (Transformation|GetWorldLocation _pill))
  (Variables|Default|SetDefaultPillZLocation (.z (Transformation|GetWorldLocation (Variables|Default|GetPill))))
  (bind (_direction _rotation _position) (Timeline|PillAnimation Play)
    (:Update
      (Transformation|SetWorldLocationAndRotation _pill (Math|Vector|MakeVector (.x _returnvalue) (.y _returnvalue) (+ (Variables|Default|GetDefaultPillZLocation) _position)) (Math|Rotator|MakeRotator 0.0 0.0 _rotation) false false))))

(fn ConstructionScript)