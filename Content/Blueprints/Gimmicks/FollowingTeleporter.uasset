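; Gimmick with a teleporter that rises after the player enters a trigger and sends any player it touches to a set destination.
; TriggerMove starts a Speed-scaled timeline that lifts the Teleporter along Z from its starting position, resetting it when finished.
; Box overlap moves the actor returned by GetOverlappedPlayerMessage to TeleportDestination, keeping rotation and scale, then stops and resets the Teleporter.
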(event OnComponentBeginOverlap(Box)
  (params (OverlappedComponent :type Primitive%20Component%20Object%20Reference) (OtherActor :type Actor%20Object%20Reference) (OtherComp :type Primitive%20Component%20Object%20Reference) (OtherBodyIndex :type Integer) (bFromSweep :type Boolean) (SweepResult :type Hit%20Result%20Structure%20%28by%20ref%29))
  (if (Actor|ActorHasTag OtherActor "Player")
    (bind _player (Class|BPIPlayerEvents|GetOverlappedPlayer(Message) OtherActor))
    (Transformation|SetActorTransform _player (Math|Transform|MakeTransform (Variables|Default|GetTeleportDestination) (.rotation (Transformation|GetActorTransform _player)) (.scale (Transformation|GetActorTransform _player))) false true)
    (CallFunction|StopMovingandResetPosition)))

(event OnComponentBeginOverlap(TriggerMove)
  (params (OverlappedComponent :type Primitive%20Component%20Object%20Reference) (OtherActor :type Actor%20Object%20Reference) (OtherComp :type Primitive%20Component%20Object%20Reference) (OtherBodyIndex :type Integer) (bFromSweep :type Boolean) (SweepResult :type Hit%20Result%20Structure%20%28by%20ref%29))
  (if (and (Actor|ActorHasTag OtherActor "Player") (not (Variables|Default|Get%20IsMoving?)))
    (CallFunction|StartMoving)))

(event Custom|StartMoving
  (bind _defaultposition (Variables|Default|GetDefaultPosition))
  (Variables|Default|Set%20IsMoving? true)
  (bind _alpha (Timeline|MovementTimeline PlayFromStart)
    (:Update
      (Transformation|SetRelativeLocation (Variables|Default|GetTeleporter) (Math|Vector|Lerp(Vector) (Variables|Default|GetDefaultPosition) (Math|Vector|MakeVector (.x _defaultposition) (.y _defaultposition) (+ 5e+03 (.z _defaultposition))) _alpha) false false))
    (:Finished
      (CallFunction|StopMovingandResetPosition))))

(event Custom|StopMovingAndResetPosition
  (Audio|Components|Audio|Stop (Variables|Default|GetMovementTimeline))
  (Transformation|SetRelativeLocation (Variables|Default|GetTeleporter) (Variables|Default|GetDefaultPosition) false false)
  (Variables|Default|Set%20IsMoving? false))

(event EventBeginPlay
  (Variables|Default|SetDefaultPosition (Variables|/Script/Engine.SceneComponent|GetRelativeLocation (Variables|Default|GetTeleporter)))
  (Components|Timeline|SetPlayRate (Variables|Default|GetMovementTimeline) (/ (Variables|Default|GetSpeed) 1e+01)))

(fn ConstructionScript)