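; A trigger-box gimmick that teleports the player to a set destination on contact.
; When an actor tagged Player overlaps the box, it fetches the player reference through message calls, disables movement and stops it immediately.
; It then moves the overlapped player to TeleportDestination, keeping rotation and scale, and re-enables movement after a short delay.
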(event OnComponentBeginOverlap(Box)
  (params (OverlappedComponent :type Primitive%20Component%20Object%20Reference) (OtherActor :type Actor%20Object%20Reference) (OtherComp :type Primitive%20Component%20Object%20Reference) (OtherBodyIndex :type Integer) (bFromSweep :type Boolean) (SweepResult :type Hit%20Result%20Structure%20%28by%20ref%29))
  (if (Actor|ActorHasTag OtherActor "Player")
    (bind _player (Class|BPIPlayerEvents|GetOverlappedPlayer(Message) OtherActor))
    (bind _playerreference (Class|BPIPlayerEvents|GetPlayerReference(Message) _player))
    (Variables|/Game/Blueprints/Player/BP_Player.BP_Player_C|SetIsAbleToMove? _playerreference false)
    (Components|Movement|StopMovementImmediately (Variables|/Script/Engine.Character|GetCharacterMovement _playerreference))
    (Transformation|SetActorTransform _player (Math|Transform|MakeTransform (Variables|Default|GetTeleportDestination) (.rotation (Transformation|GetActorTransform _player)) (.scale (Transformation|GetActorTransform _player))) false true)
    (Utilities|FlowControl|Delay 2.5)
    (Variables|/Game/Blueprints/Player/BP_Player.BP_Player_C|SetIsAbleToMove? _playerreference true)))

(fn ConstructionScript)