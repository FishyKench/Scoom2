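; A fake checkpoint gimmick that celebrates like a checkpoint when first overlapped, then reveals itself as a joke.
; The one-shot box overlap plays a timeline that spins and squishes the flag, swaps its material and fires confetti.
; Two seconds later the flag mesh switches to physics and is launched away.
; A parallel timeline raises and scales the revealed text, changing it to "SIKE!" partway through.
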(event OnComponentBeginOverlap(Box)
  (params (OverlappedComponent :type Primitive%20Component%20Object%20Reference) (OtherActor :type Actor%20Object%20Reference) (OtherComp :type Primitive%20Component%20Object%20Reference) (OtherBodyIndex :type Integer) (bFromSweep :type Boolean) (SweepResult :type Hit%20Result%20Structure%20%28by%20ref%29))
  (bind _staticmesh (Variables|Default|GetStaticMesh))
  (bind _textrender (Variables|Default|GetTextRender))
  (bind _staticmesh_2 (Variables|Default|GetStaticMesh))
  (bind _returnvalue (Transformation|GetRelativeTransform _staticmesh))
  (bind _returnvalue_2 (Transformation|GetWorldLocation _textrender))
  (Class|BPIPlayerEvents|GetPlayerReference(Message) OtherActor)
  (Utilities|FlowControl|DoOnce false
    (:Completed
      (Utilities|FlowControl|Sequence
        (:then_0
          (bind (_direction _squish _rotate) (Timeline|flag%20rotate%20and%20squish Play)
            (:Update
              (Transformation|SetRelativeTransform (Variables|Default|GetStaticMesh) (Math|Transform|MakeTransform (.location _returnvalue) (Math|Rotator|MakeRotator (.roll (.rotation _returnvalue)) (.pitch (.rotation _returnvalue)) _rotate) (Math|Vector|MakeVector (.x (.scale _returnvalue)) (.y (.scale _returnvalue)) _squish)) false false)
              (Rendering|Material|SetMaterial (Variables|Default|GetStaticMesh) 0 "/Game/Assets/NewTGR/materials/FlagOn.FlagOn")
              (Utilities|FlowControl|DoOnce false
                (:Completed
                  (Components|Activation|Activate (Variables|Default|GetNI_Confetti) false)
                  (Utilities|FlowControl|Delay 2.0)
                  (Physics|SetSimulatePhysics _staticmesh_2 true)
                  (Physics|SetPhysicsLinearVelocity _staticmesh_2 "244.000000,255.000000,225.000000" false "None"))))))
        (:then_1
          (Rendering|SetVisibility (Variables|Default|GetTextRender) true false)
          (bind (_direction_2 _scale _movement _switchtextalpha) (Timeline|Text%20anim Play)
            (:Update
              (Transformation|SetWorldTransform _textrender (Math|Transform|MakeTransform (Math|Vector|MakeVector (.x _returnvalue_2) (.y _returnvalue_2) (+ (.z _returnvalue_2) _movement)) "0, 0, 0" (Math|Conversions|ToVector(Float) _scale)) false false)
              (if (> _switchtextalpha 0.0)
                (Rendering|Components|TextRender|SetText (Variables|Default|GetTextRender) (Utilities|Text|FormatText "SIKE!"))))))))))

(fn ConstructionScript)