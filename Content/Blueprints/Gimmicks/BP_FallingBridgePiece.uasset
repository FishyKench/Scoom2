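; A falling bridge piece gimmick that drops away when an actor tagged Player overlaps its trigger.
; The overlap turns on physics simulation for the bridge mesh and disables the trigger's collision so it fires only once.
; The SizeDown timeline then drives the mesh's uniform world scale, and the actor destroys itself when the timeline finishes.
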(event OnComponentBeginOverlap(Trigger)
  (params (OverlappedComponent :type Primitive%20Component%20Object%20Reference) (OtherActor :type Actor%20Object%20Reference) (OtherComp :type Primitive%20Component%20Object%20Reference) (OtherBodyIndex :type Integer) (bFromSweep :type Boolean) (SweepResult :type Hit%20Result%20Structure%20%28by%20ref%29))
  (if (Actor|ActorHasTag OtherActor "Player")
    (Physics|SetSimulatePhysics (Variables|Default|GetFallingBridgeMesh) true)
    (Collision|SetCollisionEnabled (Variables|Default|GetTrigger) "NoCollision")
    (bind _alpha (Timeline|SizeDown Play)
      (:Update
        (Transformation|SetWorldScale3D (Variables|Default|GetFallingBridgeMesh) (Math|Conversions|ToVector(Float) _alpha)))
      (:Finished
        (Actor|DestroyActor)))))

(fn ConstructionScript)