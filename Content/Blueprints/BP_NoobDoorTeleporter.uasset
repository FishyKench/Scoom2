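; BP_NoobDoorTeleporter is a key-gated door portal that teleports the player to a set destination.
; When HasKey is true, a box overlap by a Player-tagged actor moves the actor returned by GetOverlappedPlayerMessage to TeleportDestination, preserving rotation and scale.
; The portal visual starts hidden and is revealed by a separate ActivatePortalVisual event, independent of the key check.
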(event OnComponentBeginOverlap(Box)
  (params (OverlappedComponent :type Primitive%20Component%20Object%20Reference) (OtherActor :type Actor%20Object%20Reference) (OtherComp :type Primitive%20Component%20Object%20Reference) (OtherBodyIndex :type Integer) (bFromSweep :type Boolean) (SweepResult :type Hit%20Result%20Structure%20%28by%20ref%29))
  (if (Variables|Default|GetHasKey?)
    (if (Actor|ActorHasTag OtherActor "Player")
      (bind _player (Class|BPIPlayerEvents|GetOverlappedPlayer(Message) OtherActor))
      (Transformation|SetActorTransform _player (Math|Transform|MakeTransform (Variables|Default|GetTeleportDestination) (.rotation (Transformation|GetActorTransform _player)) (.scale (Transformation|GetActorTransform _player))) false true))))

(event Custom|ActivatePortalVisual
  (Development|SetHiddeninGame (Variables|Default|GetPortalVisual) false false))

(event EventBeginPlay
  (Development|SetHiddeninGame (Variables|Default|GetPortalVisual) true false))

(fn ConstructionScript)