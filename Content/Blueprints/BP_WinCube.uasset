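; BP_WinCube is a pickup cube that triggers the win state when the player touches it.
; A Timeline started on BeginPlay drives the cube's height offset from its initial Z and its yaw.
; A box overlap with a "Player"-tagged actor fires once, calls Win on BP_ThirdPersonGameMode, plays a pickup sound at the world origin and destroys the cube.
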(event OnComponentBeginOverlap(Box)
  (params (OverlappedComponent :type Primitive%20Component%20Object%20Reference) (OtherActor :type Actor%20Object%20Reference) (OtherComp :type Primitive%20Component%20Object%20Reference) (OtherBodyIndex :type Integer) (bFromSweep :type Boolean) (SweepResult :type Hit%20Result%20Structure%20%28by%20ref%29))
  (if (Actor|ActorHasTag OtherActor "Player")
    (Utilities|FlowControl|DoOnce false
      (:Completed
        (bind _asbp_third_person_game_mode (Utilities|Casting|CastToBP_ThirdPersonGameMode (Game|GetGameMode)))
        (Default|Win _asbp_third_person_game_mode)
        (Audio|PlaySoundatLocation "/Game/SFX/PillyPickUp.PillyPickUp" "0, 0, 0" "0, 0, 0" 1.0 1.0 0.0 0 0 0 0)
        (Actor|DestroyActor)))))

(event EventBeginPlay
  (bind _wincube (Variables|Default|GetWinCube))
  (bind _returnvalue (Transformation|GetWorldLocation _wincube))
  (Variables|Default|SetDefaultCubeZLocation (.z (Transformation|GetWorldLocation (Variables|Default|GetWinCube))))
  (bind (_direction _rotation _position) (Timeline|Timeline Play)
    (:Update
      (Transformation|SetWorldLocationAndRotation _wincube (Math|Vector|MakeVector (.x _returnvalue) (.y _returnvalue) (+ (Variables|Default|GetDefaultCubeZLocation) _position)) (Math|Rotator|MakeRotator 0.0 0.0 _rotation) false false))))

(fn ConstructionScript)