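; BP_HalfPill is a half-pill pickup that the player collects by touching it.
; From BeginPlay, a Timeline drives the mesh's height around its starting Z and its yaw to animate it.
; Sphere overlap by a "Player"-tagged actor increments the half-pill count in BP_ThirdPersonGameMode, plays a pickup sound at world origin, and destroys the pickup after a short delay.
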(event OnComponentBeginOverlap(Sphere)
  (params (OverlappedComponent :type Primitive%20Component%20Object%20Reference) (OtherActor :type Actor%20Object%20Reference) (OtherComp :type Primitive%20Component%20Object%20Reference) (OtherBodyIndex :type Integer) (bFromSweep :type Boolean) (SweepResult :type Hit%20Result%20Structure%20%28by%20ref%29))
  (if (Actor|ActorHasTag OtherActor "Player")
    (bind _asbp_third_person_game_mode (Utilities|Casting|CastToBP_ThirdPersonGameMode (Game|GetGameMode)))
    (Default|IncreaseHalfpillAmount _asbp_third_person_game_mode)
    (Audio|PlaySoundatLocation "/Game/SFX/PillyPickUp.PillyPickUp" "0, 0, 0" "0, 0, 0" 1.0 1.0 0.0 0 0 0 0)
    (Utilities|FlowControl|Delay 0.1)
    (Actor|DestroyActor)))

(event EventBeginPlay
  (bind _halfpillmesh (Variables|Default|GetHalfPillMesh))
  (bind _returnvalue (Transformation|GetWorldLocation _halfpillmesh))
  (Variables|Default|SetDefaultPillZLocation (.z (Transformation|GetWorldLocation (Variables|Default|GetHalfPillMesh))))
  (bind (_direction _rotation _position) (Timeline|Timeline Play)
    (:Update
      (Transformation|SetWorldLocationAndRotation _halfpillmesh (Math|Vector|MakeVector (.x _returnvalue) (.y _returnvalue) (+ (Variables|Default|GetDefaultPillZLocation) _position)) (Math|Rotator|MakeRotator 0.0 0.0 _rotation) false false))))

(fn ConstructionScript)